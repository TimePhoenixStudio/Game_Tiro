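; BP_Character is a base character Blueprint that manages sprinting and the movement speed that goes with it.
; StartSprinting runs only when the character is neither aiming nor crouching, while StopSprinting always returns to normal speed.
; Both events update the sprint flag, fire a matching start or stop notification, and call SetCharacterSpeed.
; SetCharacterSpeed selects Max Walk Speed from MovementSpeed values for normal, sprinting and crouching states.
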(event `Start Sprinting`
  (if (`KismetMathLibrary.BooleanNOR` (`self.Is Aiming?`) (`self.Is Crounching?`))
    (set `self.Is Isprinting?` true)
    (`self.On Start Sprinting`)
    (`self.Set Character Speed` "NewEnumerator1")))

(event `Stop Sprinting`
  (set `self.Is Isprinting?` false)
  (`self.On Stop Sprinting`)
  (`self.Set Character Speed` "NewEnumerator0"))

(fn `Set Character Speed`
  (params (`New Speed` :type "/Game/Blueprints/Base/Characters/E_MovementSpeed Enum" :default "NewEnumerator0"))
  (bind (_movement_speed_normal _movement_speed_sprinting _movement_speed_crounching) (break `/Game/Blueprints/Base/Characters/STR_MovementSpeed` (`self.Movement Speed`)))
  (set `CharacterMovementComponent.MaxWalkSpeed` (select `/Game/Blueprints/Base/Characters/E_MovementSpeed` `New Speed` :`NewEnumerator0` _movement_speed_normal :`NewEnumerator1` _movement_speed_sprinting :`NewEnumerator2` _movement_speed_crounching) (`self.CharacterMovement`)))

(fn `UserConstructionScript`)